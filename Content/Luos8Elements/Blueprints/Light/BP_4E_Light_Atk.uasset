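; BP_4E_Light_Atk is a Light attack actor that damages what its Sphere component hits.
; On a component hit, it runs a debug-drawn Visibility sphere trace at the sphere's location as a gate.
; If the trace finds anything, it applies fixed damage to the hit actor unless tagged Player, then destroys itself either way.
; The trace result only gates this logic; damage targets the collision's OtherActor.
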(event `self.Sphere.OnComponentHit`
  (params (HitComponent :type "PrimitiveComponent Object Reference") (OtherActor :type "Actor Object Reference") (OtherComp :type "PrimitiveComponent Object Reference") (NormalImpulse :type "Vector Structure") (Hit :type "HitResult Structure (by ref)"))
  (bind _returnvalue (`SceneComponent.K2_GetComponentLocation` (`self.Sphere`)))
  ;[1 1 1] AttackTrace when SpheregotHit and Apply DMG
  (bind (_outhit _returnvalue_2) (`KismetSystemLibrary.SphereTraceSingle` :`Start` _returnvalue :`End` _returnvalue :`Radius` 100.0 :`TraceChannel` "TraceTypeQuery1" :`DrawDebugType` "ForDuration"))
  (if _returnvalue_2
    (if (not (`self.ActorHasTag` OtherActor "Player"))
      (`GameplayStatics.ApplyDamage` OtherActor 50.0))
    (`self.K2_DestroyActor`)))

(fn `UserConstructionScript`
  (`parent.UserConstructionScript`))