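; Level 3 lizard warrior enemy that patrols around a point, fights the player and drops a key on death.
; Sight, noise-area overlap or damage triggers a one-time intro montage, then a MoveTo chase with two random attacks.
; AttackTrace sphere-traces to damage the player; incoming damage loses a flat 20, and criticals pause new movement orders.
; Tick drives health regen, health widget values and the combat alert icon.
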(event `PlayerRespawn`
  (bind _returnvalue (`GameplayStatics.GetPlayerCharacter` 0))
  (`|ExecutionSequence`
    (:`then_0`
      (bind _asthird_person_character_bp (cast `/Game/_ProjectContent/Blueprint/ThirdPersonCharacter_BP` _returnvalue))
      (set `self.PlayerRef` _asthird_person_character_bp)
      (bind _asai_health_ui (cast `/Game/_ProjectContent/Widget/AI_HealthUI` (`WidgetComponent.GetUserWidgetObject` (`self.AiHealthWidget`))))
      (set `self.HealthWidgetRef` _asai_health_ui)
      (cast `/Game/_ProjectContent/Widget/AI_Stats_AlertUI` (`WidgetComponent.GetUserWidgetObject` (`self.Ai_State_Alert`))))
    (:`then_1`
      (bind _asthird_person_character_bp_2 (cast `/Game/_ProjectContent/Blueprint/ThirdPersonCharacter_BP` _returnvalue))
      (set `/Game/_ProjectContent/Blueprint/ThirdPersonCharacter_BP.Lizard_Ai3_Ref` self _asthird_person_character_bp_2))
    (:`then_2`
      (`self.Partroling` :!label _label)
      (set `self.AttackingPlayer` false))))

(event `self.ReceiveBeginPlay`
  (goto _label))

(event `self.Sphere.OnComponentBeginOverlap`
  (params (OverlappedComponent :type "PrimitiveComponent Object Reference") (OtherActor :type "Actor Object Reference") (OtherComp :type "PrimitiveComponent Object Reference") (OtherBodyIndex :type Integer) (bFromSweep :type Boolean) (SweepResult :type "HitResult Structure (by ref)"))
  ;[1 1 1] Visibility Check Widget AI_Health
  (cast `/Game/_ProjectContent/Blueprint/ThirdPersonCharacter_BP` OtherActor)
  (`SceneComponent.SetVisibility` (`self.AiHealthWidget`) true false))

(event `self.Sphere.OnComponentEndOverlap`
  (params (OverlappedComponent :type "PrimitiveComponent Object Reference") (OtherActor :type "Actor Object Reference") (OtherComp :type "PrimitiveComponent Object Reference") (OtherBodyIndex :type Integer))
  ;[1 1 1] Visibility Check Widget AI_Health
  (cast `/Game/_ProjectContent/Blueprint/ThirdPersonCharacter_BP` OtherActor)
  (`SceneComponent.SetVisibility` (`self.AiHealthWidget`) false false))

(event `self.ReceiveTick`
  (params (DeltaSeconds :type "Float (single-precision)"))
  (bind _ai_state_alert (`self.Ai_State_Alert`))
  (bind _healthwidgetref (`self.HealthWidgetRef`))
  (`|ExecutionSequence`
    (:`then_0`
      ;[1 1 1] Set Health var in AiHealth widget
      (set `/Game/_ProjectContent/Widget/AI_HealthUI.Health` (`self.HealthCurrent`) _healthwidgetref)
      (set `/Game/_ProjectContent/Widget/AI_HealthUI.Level` (`self.EnemyLevel`) _healthwidgetref))
    (:`then_1`
      ;[1 1 1] Health Regen
      (if (< (`self.HealthCurrent`) (`self.MaxHealth`))
        (`KismetSystemLibrary.Delay` 0.5)
        (set `self.HealthCurrent` (+ (`self.HealthCurrent`) 0.5))))
    (:`then_2`
      ;[1 1 1] Set AlertWidget
      (if (`self.AttackingPlayer`)
        (`SceneComponent.SetVisibility` _ai_state_alert true false)
        (else
          (`SceneComponent.SetVisibility` _ai_state_alert false false))))))

(event `self.ReceiveAnyDamage`
  (params (Damage :type "Float (single-precision)") (DamageType :type "DamageType Object Reference") (InstigatedBy :type "Controller Object Reference") (DamageCauser :type "Actor Object Reference"))
  ;[1 1 1] Health Reduce
  (set `self.HealthCurrent` (- (`self.HealthCurrent`) (- Damage 20.0)))
  (if (< (`self.HealthCurrent`) 0.0)
    (`/Engine/EditorBlueprintResources/StandardMacros.DoOnce` false
      (:`Completed`
        (set `self.IsDead?` true)
        (set `CharacterMovementComponent.MaxWalkSpeed` 0.0 (`self.CharacterMovement`))
        (`PrimitiveComponent.SetCollisionEnabled` (`self.CapsuleComponent`) "NoCollision")
        ;[1 1 1] Spawn Key
        (`/Engine/EditorBlueprintResources/StandardMacros.DoOnce` false
          (:`Completed`
            (`|SpawnActorFromClass` "/Game/_ProjectContent/Blueprint/Item/Key_BP.Key_BP_C" (`KismetMathLibrary.MakeTransform` (- (.location (`self.GetTransform`)) (0.0 0.0 80.0)) (.rotation (`self.GetTransform`)) (.scale (`self.GetTransform`))) "Undefined" "OverrideRootScale" null null)
            (`KismetSystemLibrary.Delay` 3.0)
            (`self.K2_DestroyActor`)))))
    (else
      (`|ExecutionSequence`
        (:`then_0`
          (if (not (`self.HasAttackedFromPlayer`))
            (set `self.HasAttackedFromPlayer` true)
            (`KismetSystemLibrary.Delay` 0.5)
            (set `self.HasAttackedFromPlayer` false)))
        (:`then_1`
          ;[1 1 1] Seeing Pawn and Entrance Combat
          (if (not (`self.IsDead?`)) :!label _label_2
            (if (not (`self.EntranceCombat?`)) :!label _label_3
              (`/Engine/EditorBlueprintResources/StandardMacros.DoOnce` false
                (:`Completed`
                  (set `CharacterMovementComponent.MaxWalkSpeed` 0.0 (`self.CharacterMovement`))
                  (`|PlayMontage` (`self.Mesh`) "/Game/LizardWarrior/Animations/Lizard_Generic_MT.Lizard_Generic_MT" 0.5 0.0 "Lizard_Spell"
                    (:`OnCompleted`
                      (set `self.EntranceCombat?` true))))))
            (set `self.AttackingPlayer` true)
            (set `CharacterMovementComponent.MaxWalkSpeed` 400.0 (`self.CharacterMovement`))
            (`self.AttackPlayer`)))
        (:`then_2`
          (if (`self.GetCritical?`)
            (`|SpawnActorFromClass` "/Game/Luos8Elements/Blueprints/Light/BP_Light_DMG.BP_Light_DMG_C" (`KismetMathLibrary.Conv_VectorToTransform` (`SceneComponent.K2_GetComponentLocation` (`self.DMG_effect`))) "Undefined" "OverrideRootScale" null null)
            (`|ExecutionSequence`
              (:`then_0`
                (bind _output_get (set `self.RecoverRate` 3.0))
                (set `self.GetCritical?` false)
                (set `self.CanMove?` false))
              (:`then_1`
                (`KismetSystemLibrary.Delay` _output_get)
                (set `self.CanMove?` true)))))))))

(event `self.PawnSensing.OnSeePawn`
  (params (Pawn :type "Pawn Object Reference"))
  ;[1 1 1] Seeing Pawn and Entrance Combat
  (goto _label_2))

(event `self.NoiseDetectArea.OnComponentBeginOverlap`
  (params (OverlappedComponent :type "PrimitiveComponent Object Reference") (OtherActor :type "Actor Object Reference") (OtherComp :type "PrimitiveComponent Object Reference") (OtherBodyIndex :type Integer) (bFromSweep :type Boolean) (SweepResult :type "HitResult Structure (by ref)"))
  ;[1 1 1] Seeing Pawn and Entrance Combat
  (cast `/Game/_ProjectContent/Blueprint/ThirdPersonCharacter_BP` OtherActor)
  (goto _label_3))

(event `Partroling`
  ;[1 1 1] AI Partroling
  (if (`self.CanMove?`)
    (if (`self.Moving?`)
      _
      (elif (`self.AttackingPlayer`)
        (`self.AttackPlayer`)
        (else
          (`|AIMoveTo` self (`NavigationSystemV1.K2_GetRandomLocationInNavigableRadius` (`self.K2_GetActorLocation` (`self.PartrolPoint`)) (`self.PartrolRadius`) null null) null
            (:`then`
              (set `self.Moving?` true))
            (:`OnSuccess`
              (`KismetSystemLibrary.Delay` (`KismetMathLibrary.RandomFloatInRange` 1.0 3.0))
              (set `self.Moving?` false)
              (if (not (`self.IsDead?`)) :!label _label_4
                (`self.Partroling`)))
            (:`OnFail`
              (set `self.Moving?` false)
              (goto _label_4))))))))

(event `AttackPlayer`
  ;[1 1 1] AI Attack Player
  (if (`self.CanMove?`)
    (`|AIMoveTo` self (0.0 0.0 0.0) (`GameplayStatics.GetPlayerCharacter` 0) (`self.PlayerVicinity`)
      (:`then`
        (`self.FacePlayer`))
      (:`OnSuccess`
        (if (not (`self.HasAttack?`))
          (set `self.HasAttack?` true)
          (set `CharacterMovementComponent.MaxWalkSpeed` 0.0 (`self.CharacterMovement`))
          (switch `int` (`KismetMathLibrary.RandomIntegerInRange` 0 1)
            (:`0`
              (set `self.Attack1` true)
              (set `self.AttackMode` 0)
              (`KismetSystemLibrary.Delay` 1.0)
              (set `self.Attack1` false))
            (:`1`
              (set `self.Attack2` true)
              (set `self.AttackMode` 1)
              (`KismetSystemLibrary.Delay` 1.0)
              (set `self.Attack2` false)))
          (set `CharacterMovementComponent.MaxWalkSpeed` 400.0 (`self.CharacterMovement`))
          (`KismetSystemLibrary.Delay` (`self.RecoverRate`))
          (set `self.RecoverRate` 0.0)
          (set `self.HasAttack?` false)))
      (:`OnFail`
        (`self.AttackPlayer`)))))

(event `AttackTrace`
  (bind _returnvalue (`GameplayStatics.GetPlayerCharacter` 0))
  (bind _attackform (`self.AttackForm`))
  (bind _returnvalue_2 (`SceneComponent.K2_GetComponentLocation` _attackform))
  ;[1 1 1] AttackTrace And Apply DMG
  (bind _outhit (`KismetSystemLibrary.SphereTraceSingle` _returnvalue_2 (+ _returnvalue_2 (* (`SceneComponent.GetForwardVector` _attackform) (`self.AttackRange`))) 35.0 "TraceTypeQuery1"))
  (if (`GameplayStatics.BreakHitResult` _outhit)
    (switch `int` (`self.AttackMode`)
      (:`0`
        (`GameplayStatics.ApplyDamage` _returnvalue (`self.ATKDMG1`)))
      (:`1`
        (`GameplayStatics.ApplyDamage` _returnvalue (`self.ATKDMG2`))))))

(event `FacePlayer`
  ;[1 1 1] AI Face on Player
  (if (not (`self.IsDead?`))
    (if (`self.HasAttack?`)
      (`self.K2_SetActorRotation` (`KismetMathLibrary.MakeRotator` 0.0 0.0 (.yaw (`KismetMathLibrary.FindLookAtRotation` (`SceneComponent.K2_GetComponentLocation` (`self.Mesh`)) (`self.K2_GetActorLocation` (`self.PlayerRef`)))))))
    (`KismetSystemLibrary.RetriggerableDelay` 0.5)
    (`self.FacePlayer`)))

(fn `UserConstructionScript`)