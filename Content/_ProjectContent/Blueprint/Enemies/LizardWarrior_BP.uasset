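; Lizard warrior enemy that patrols random points around a patrol point, then chases and attacks the player once it sees or is hurt.
; Movement runs on self-recalling AIMoveTo events, with two random attacks on a recovery cooldown.
; AttackTrace sphere-traces forward, and any blocking hit damages the player pawn.
; Tick feeds regenerating health to a proximity-shown widget; death disables collision and destroys the actor after a delay.
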(event `self.ReceiveBeginPlay`
  (`|ExecutionSequence`
    (:`then_0`
      (bind _asthird_person_character_bp (cast `/Game/_ProjectContent/Blueprint/ThirdPersonCharacter_BP` (`GameplayStatics.GetPlayerCharacter` 0)))
      (set `self.PlayerRef` _asthird_person_character_bp)
      (bind _asai_health_ui (cast `/Game/_ProjectContent/Widget/AI_HealthUI` (`WidgetComponent.GetUserWidgetObject` (`self.AiHealthWidget`))))
      (set `self.HealthWidgetRef` _asai_health_ui))
    (:`then_1`
      (`self.Partroling`))))

(event `self.Sphere.OnComponentBeginOverlap`
  (params (OverlappedComponent :type "PrimitiveComponent Object Reference") (OtherActor :type "Actor Object Reference") (OtherComp :type "PrimitiveComponent Object Reference") (OtherBodyIndex :type Integer) (bFromSweep :type Boolean) (SweepResult :type "HitResult Structure (by ref)"))
  ;[1 1 1] Visibility Check Widget AI_Health
  (cast `/Game/_ProjectContent/Blueprint/ThirdPersonCharacter_BP` OtherActor)
  (`SceneComponent.SetVisibility` (`self.AiHealthWidget`) true false))

(event `self.Sphere.OnComponentEndOverlap`
  (params (OverlappedComponent :type "PrimitiveComponent Object Reference") (OtherActor :type "Actor Object Reference") (OtherComp :type "PrimitiveComponent Object Reference") (OtherBodyIndex :type Integer))
  ;[1 1 1] Visibility Check Widget AI_Health
  (cast `/Game/_ProjectContent/Blueprint/ThirdPersonCharacter_BP` OtherActor)
  (`SceneComponent.SetVisibility` (`self.AiHealthWidget`) false false))

(event `self.ReceiveTick`
  (params (DeltaSeconds :type "Float (single-precision)"))
  (`|ExecutionSequence`
    (:`then_0`
      ;[1 1 1] Set Health var in AiHealth widget
      (set `/Game/_ProjectContent/Widget/AI_HealthUI.Health` (`self.HealthCurrent`) (`self.HealthWidgetRef`)))
    (:`then_1`
      ;[1 1 1] Health Regen
      (if (< (`self.HealthCurrent`) (`self.MaxHealth`))
        (`KismetSystemLibrary.Delay` 0.5)
        (set `self.HealthCurrent` (+ (`self.HealthCurrent`) 0.5))))))

(event `self.ReceiveAnyDamage`
  (params (Damage :type "Float (single-precision)") (DamageType :type "DamageType Object Reference") (InstigatedBy :type "Controller Object Reference") (DamageCauser :type "Actor Object Reference"))
  ;[1 1 1] Health Reduce
  (set `self.HealthCurrent` (- (`self.HealthCurrent`) Damage))
  (if (< (`self.HealthCurrent`) 0.0)
    (set `self.IsDead?` true)
    (set `CharacterMovementComponent.MaxWalkSpeed` 0.0 (`self.CharacterMovement`))
    (`PrimitiveComponent.SetCollisionEnabled` (`self.CapsuleComponent`) "NoCollision")
    (`KismetSystemLibrary.Delay` 3.0)
    (`self.K2_DestroyActor`)
    (else
      (`|ExecutionSequence`
        (:`then_0`
          (if (not (`self.HasAttackedFromPlayer`))
            (set `self.HasAttackedFromPlayer` true)
            (`KismetSystemLibrary.Delay` 0.5)
            (set `self.HasAttackedFromPlayer` false)
            ;[1 1 1] Seeing Pawn
            (set `self.AttackingPlayer` true :!label _label)
            (set `CharacterMovementComponent.MaxWalkSpeed` 400.0 (`self.CharacterMovement`))
            (`self.AttackPlayer`)))
        (:`then_1`
          (goto _label))))))

(event `self.PawnSensing.OnSeePawn`
  (params (Pawn :type "Pawn Object Reference"))
  ;[1 1 1] Seeing Pawn
  (if (not (`self.IsDead?`))
    (goto _label)))

(event `Partroling`
  ;[1 1 1] AI Partroling
  (if (`self.Moving?`)
    _
    (elif (`self.AttackingPlayer`)
      (`self.AttackPlayer`)
      (else
        (`|AIMoveTo` self (`NavigationSystemV1.K2_GetRandomLocationInNavigableRadius` (`self.K2_GetActorLocation` (`self.PartrolPoint`)) (`self.PartrolRadius`) null null) null
          (:`then`
            (set `self.Moving?` true))
          (:`OnSuccess`
            (`KismetSystemLibrary.Delay` (`KismetMathLibrary.RandomFloatInRange` 1.0 3.0))
            (set `self.Moving?` false)
            (if (not (`self.IsDead?`)) :!label _label_2
              (`self.Partroling`)))
          (:`OnFail`
            (set `self.Moving?` false)
            (goto _label_2)))))))

(event `AttackPlayer`
  ;[1 1 1] AI Attack Player
  (`|AIMoveTo` self (0.0 0.0 0.0) (`GameplayStatics.GetPlayerCharacter` 0) (`self.PlayerVicinity`)
    (:`then`
      (`self.FacePlayer`))
    (:`OnSuccess`
      (if (not (`self.HasAttack?`))
        (set `self.HasAttack?` true)
        (set `CharacterMovementComponent.MaxWalkSpeed` 0.0 (`self.CharacterMovement`))
        (switch `int` (`KismetMathLibrary.RandomIntegerInRange` 0 1)
          (:`0`
            (set `self.Attack1` true)
            (set `self.AttackMode` 0)
            (`KismetSystemLibrary.Delay` 1.0)
            (set `self.Attack1` false))
          (:`1`
            (set `self.Attack2` true)
            (set `self.AttackMode` 1)
            (`KismetSystemLibrary.Delay` 1.0)
            (set `self.Attack2` false)))
        (set `CharacterMovementComponent.MaxWalkSpeed` 400.0 (`self.CharacterMovement`))
        (`KismetSystemLibrary.Delay` (`self.RecoverRate`))
        (set `self.HasAttack?` false)))
    (:`OnFail`
      (`self.AttackPlayer`))))

(event `AttackTrace`
  (bind _returnvalue (`GameplayStatics.GetPlayerPawn` 0))
  (bind _attackform (`self.AttackForm`))
  (bind _returnvalue_2 (`SceneComponent.K2_GetComponentLocation` _attackform))
  ;[1 1 1] AttackTrace And Apply DMG
  (bind _outhit (`KismetSystemLibrary.SphereTraceSingle` :`Start` _returnvalue_2 :`End` (+ _returnvalue_2 (* (`SceneComponent.GetForwardVector` _attackform) (`self.AttackRange`))) :`Radius` 35.0 :`TraceChannel` "TraceTypeQuery1" :`DrawDebugType` "ForDuration"))
  (if (`GameplayStatics.BreakHitResult` _outhit)
    (if true
      (switch `int` (`self.AttackMode`)
        (:`0`
          (`GameplayStatics.ApplyDamage` _returnvalue (`self.ATKDMG1`)))
        (:`1`
          (`GameplayStatics.ApplyDamage` _returnvalue (`self.ATKDMG2`)))))))

(event `FacePlayer`
  ;[1 1 1] AI Face on Player
  (if (not (`self.IsDead?`))
    (if (`self.HasAttack?`)
      (`self.K2_SetActorRotation` (`KismetMathLibrary.MakeRotator` 0.0 0.0 (.yaw (`KismetMathLibrary.FindLookAtRotation` (`SceneComponent.K2_GetComponentLocation` (`self.Mesh`)) (`self.K2_GetActorLocation` (`self.PlayerRef`)))))))
    (`KismetSystemLibrary.RetriggerableDelay` 0.5)
    (`self.FacePlayer`)))

(fn `UserConstructionScript`)