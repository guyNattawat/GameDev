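; Ammo generator pickup that spawns a magic ammo actor at its Arrow on BeginPlay and lets the player collect it.
; Box overlap toggles player input and a Gate, so Interact works only nearby.
; A pickup, allowed below the ammo cap while available, increments the character's MagicAmmo, plays a sound and destroys the spawned actor.
; A DoOnce with no visible reset then triggers a delayed respawn, so that respawn fires only once.
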(event `Respawn_Ammo`
  (bind _returnvalue (`|SpawnActorFromClass` "/Game/_ProjectContent/Blueprint/Item/MagicAmmo_Interac_BP.MagicAmmo_Interac_BP_C" (`SceneComponent.K2_GetComponentToWorld` (`self.Arrow`)) "Undefined" "OverrideRootScale" null null :!label _label))
  (set `self.CanPick?` true))

(event `self.ReceiveBeginPlay`
  (goto _label))

(event `InputAction|Interact`
  (params (Key :type "Key Structure"))
  (:`Pressed`
    (bind _asthird_person_character_bp (cast `/Game/_ProjectContent/Blueprint/ThirdPersonCharacter_BP` (`GameplayStatics.GetPlayerCharacter` 0)))
    (if (< (`/Game/_ProjectContent/Blueprint/ThirdPersonCharacter_BP.MagicAmmo` _asthird_person_character_bp) 5)
      (if (`self.CanPick?`)
        (`/Engine/EditorBlueprintResources/StandardMacros.Gate` true :!label _label_2
          (:`Exit`
            (bind _asthird_person_character_bp_2 (cast `/Game/_ProjectContent/Blueprint/ThirdPersonCharacter_BP` (`GameplayStatics.GetPlayerCharacter` 0)))
            (set `self.CanPick?` false)
            (set `/Game/_ProjectContent/Blueprint/ThirdPersonCharacter_BP.MagicAmmo` (+ (`/Game/_ProjectContent/Blueprint/ThirdPersonCharacter_BP.MagicAmmo` _asthird_person_character_bp_2) 1) _asthird_person_character_bp_2)
            (`GameplayStatics.PlaySoundAtLocation` "/Game/_ProjectContent/Audio/Pick_item2_Cue.Pick_item2_Cue" (`self.K2_GetActorLocation`) (struct) 1.0 1.0 0.0 null null null)
            (`self.K2_DestroyActor` (stale `Respawn_Ammo` _returnvalue))
            (`/Engine/EditorBlueprintResources/StandardMacros.DoOnce` false
              (:`Completed`
                (`KismetSystemLibrary.Delay` 20.0)
                (`self.Respawn_Ammo`)))))))))

(event `self.Box.OnComponentBeginOverlap`
  (params (OverlappedComponent :type "PrimitiveComponent Object Reference") (OtherActor :type "Actor Object Reference") (OtherComp :type "PrimitiveComponent Object Reference") (OtherBodyIndex :type Integer) (bFromSweep :type Boolean) (SweepResult :type "HitResult Structure (by ref)"))
  (cast `/Game/_ProjectContent/Blueprint/ThirdPersonCharacter_BP` OtherActor)
  (`self.EnableInput` (`GameplayStatics.GetPlayerController` 0))
  (goto _label_2 :!via `Open`))

(event `self.Box.OnComponentEndOverlap`
  (params (OverlappedComponent :type "PrimitiveComponent Object Reference") (OtherActor :type "Actor Object Reference") (OtherComp :type "PrimitiveComponent Object Reference") (OtherBodyIndex :type Integer))
  (cast `/Game/_ProjectContent/Blueprint/ThirdPersonCharacter_BP` OtherActor)
  (`self.DisableInput` (`GameplayStatics.GetPlayerController` 0))
  (goto _label_2 :!via `Close`))

(fn `UserConstructionScript`)