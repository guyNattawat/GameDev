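; Health potion pickup that adds to the third-person character's potion count when touched.
; A box overlap casts the other actor to ThirdPersonCharacter_BP and acts only while its HealthPotion count is below two.
; On pickup it plays a sound at the player pawn's location, increments the count and destroys itself.
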(event `self.Box.OnComponentBeginOverlap`
  (params (OverlappedComponent :type "PrimitiveComponent Object Reference") (OtherActor :type "Actor Object Reference") (OtherComp :type "PrimitiveComponent Object Reference") (OtherBodyIndex :type Integer) (bFromSweep :type Boolean) (SweepResult :type "HitResult Structure (by ref)"))
  (bind _asthird_person_character_bp (cast `/Game/_ProjectContent/Blueprint/ThirdPersonCharacter_BP` OtherActor))
  (if (< (`/Game/_ProjectContent/Blueprint/ThirdPersonCharacter_BP.HealthPotion` _asthird_person_character_bp) 2)
    (`GameplayStatics.PlaySoundAtLocation` "/Game/_ProjectContent/Audio/Pick_item_Cue.Pick_item_Cue" (`self.K2_GetActorLocation` (`GameplayStatics.GetPlayerPawn` 0)) (struct) 1.0 1.0 0.0 null null null)
    (set `/Game/_ProjectContent/Blueprint/ThirdPersonCharacter_BP.HealthPotion` (+ (`/Game/_ProjectContent/Blueprint/ThirdPersonCharacter_BP.HealthPotion` _asthird_person_character_bp) 1) _asthird_person_character_bp)
    (`self.K2_DestroyActor`)))

(fn `UserConstructionScript`)