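; Key pickup actor that the player collects by pressing Interact while inside its interaction area.
; Overlapping the area enables input on the actor, and a gate opens only for the third-person character, closing again when that character leaves.
; An Interact press through the open gate increments the character's Key count, plays a pickup sound at the character's location and destroys the key.
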(event `self.Interac_Area.OnComponentBeginOverlap`
  (params (OverlappedComponent :type "PrimitiveComponent Object Reference") (OtherActor :type "Actor Object Reference") (OtherComp :type "PrimitiveComponent Object Reference") (OtherBodyIndex :type Integer) (bFromSweep :type Boolean) (SweepResult :type "HitResult Structure (by ref)"))
  (`self.EnableInput` (`GameplayStatics.GetPlayerController` 0))
  (cast `/Game/_ProjectContent/Blueprint/ThirdPersonCharacter_BP` OtherActor)
  (goto _label :!via `Open`))

(event `InputAction|Interact`
  (params (Key :type "Key Structure"))
  (:`Pressed`
    (`/Engine/EditorBlueprintResources/StandardMacros.Gate` true :!label _label
      (:`Exit`
        (bind _asthird_person_character_bp (cast `/Game/_ProjectContent/Blueprint/ThirdPersonCharacter_BP` (`GameplayStatics.GetPlayerCharacter` 0)))
        (set `/Game/_ProjectContent/Blueprint/ThirdPersonCharacter_BP.Key` (+ (`/Game/_ProjectContent/Blueprint/ThirdPersonCharacter_BP.Key` _asthird_person_character_bp) 1) _asthird_person_character_bp)
        (`GameplayStatics.PlaySoundAtLocation` "/Game/_ProjectContent/Audio/Pick_item_Cue.Pick_item_Cue" (`self.K2_GetActorLocation` _asthird_person_character_bp) (struct) 1.0 1.0 0.0 null null null)
        (`self.K2_DestroyActor`)))))

(event `self.Interac_Area.OnComponentEndOverlap`
  (params (OverlappedComponent :type "PrimitiveComponent Object Reference") (OtherActor :type "Actor Object Reference") (OtherComp :type "PrimitiveComponent Object Reference") (OtherBodyIndex :type Integer))
  (`self.DisableInput` (`GameplayStatics.GetPlayerController` 0))
  (cast `/Game/_ProjectContent/Blueprint/ThirdPersonCharacter_BP` OtherActor)
  (goto _label :!via `Close`))

(fn `UserConstructionScript`)