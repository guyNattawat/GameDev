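; Key placement spot where the player spends one key from ThirdPersonCharacter_BP to slide a stone piece downward.
; A box overlap enables Interact input and opens a gate while the character is inside, and reverses both on exit.
; A successful press drives the StoneActive timeline, lerping the KeyPlacing2 component between transforms cached at BeginPlay.
; Input is disabled during the slide, with a sliding sound at the start and a placing sound shortly after it finishes.
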(event `self.ReceiveBeginPlay`
  (bind (_returnvalue_location _returnvalue_rotation _returnvalue_scale) (`KismetMathLibrary.BreakTransform` (`SceneComponent.GetRelativeTransform` (`self.KeyPlacing2`))))
  (set `self.Out Position` (`KismetMathLibrary.MakeTransform` _returnvalue_location _returnvalue_rotation _returnvalue_scale))
  (set `self.In Position` (`KismetMathLibrary.MakeTransform` (- _returnvalue_location (0.0 0.0 55.0)) _returnvalue_rotation _returnvalue_scale)))

(event `InputAction|Interact`
  (params (Key :type "Key Structure"))
  (bind _returnvalue (`self.K2_GetActorLocation`))
  (:`Pressed`
    (bind _asthird_person_character_bp (cast `/Game/_ProjectContent/Blueprint/ThirdPersonCharacter_BP` (`GameplayStatics.GetPlayerCharacter` 0)))
    (bind _key (`/Game/_ProjectContent/Blueprint/ThirdPersonCharacter_BP.Key` _asthird_person_character_bp))
    (if (> _key 0)
      (set `/Game/_ProjectContent/Blueprint/ThirdPersonCharacter_BP.Key` (- _key 1) _asthird_person_character_bp)
      (`/Engine/EditorBlueprintResources/StandardMacros.Gate` true :!label _label
        (:`Exit`
          (`GameplayStatics.PlaySoundAtLocation` "/Game/_ProjectContent/Audio/Stone_Slide_Cue.Stone_Slide_Cue" _returnvalue (struct) 1.0 1.0 0.0 null null null)
          (bind (_direction _stoneslide) (`Timeline|StoneActive` :!via `PlayFromStart`)
            (:`Update`
              (`SceneComponent.K2_SetRelativeTransform` (`self.KeyPlacing2`) (`KismetMathLibrary.TLerp` (`self.Out Position`) (`self.In Position`) _stoneslide) false false)
              (`self.DisableInput` null))
            (:`Finished`
              (`KismetSystemLibrary.Delay` 0.2)
              (`GameplayStatics.PlaySoundAtLocation` "/Game/_ProjectContent/Audio/Placing_Spacial_Cue.Placing_Spacial_Cue" _returnvalue (struct) 1.0 1.0 0.0 null null null))))))))

(event `self.Box.OnComponentBeginOverlap`
  (params (OverlappedComponent :type "PrimitiveComponent Object Reference") (OtherActor :type "Actor Object Reference") (OtherComp :type "PrimitiveComponent Object Reference") (OtherBodyIndex :type Integer) (bFromSweep :type Boolean) (SweepResult :type "HitResult Structure (by ref)"))
  (cast `/Game/_ProjectContent/Blueprint/ThirdPersonCharacter_BP` OtherActor)
  (`self.EnableInput` (`GameplayStatics.GetPlayerController` 0))
  (goto _label :!via `Open`))

(event `self.Box.OnComponentEndOverlap`
  (params (OverlappedComponent :type "PrimitiveComponent Object Reference") (OtherActor :type "Actor Object Reference") (OtherComp :type "PrimitiveComponent Object Reference") (OtherBodyIndex :type Integer))
  (cast `/Game/_ProjectContent/Blueprint/ThirdPersonCharacter_BP` OtherActor)
  (`self.DisableInput` (`GameplayStatics.GetPlayerController` 0))
  (goto _label :!via `Close`))

(fn `UserConstructionScript`)