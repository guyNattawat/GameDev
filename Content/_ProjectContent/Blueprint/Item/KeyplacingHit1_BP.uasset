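; Rune stone actor that sinks when hit, plays a placing sound, then rises back after a pause.
; BeginPlay caches the raised and lowered relative transforms, and two timelines lerp between them, one for each direction, with slide sounds.
; A DoOnce blocks retriggering during the sequence, which calls DisableInput with the first player controller at the start and re-enables it before resetting.
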(event `self.ReceiveBeginPlay`
  (bind (_returnvalue_location _returnvalue_rotation _returnvalue_scale) (`KismetMathLibrary.BreakTransform` (`SceneComponent.GetRelativeTransform` (`self.SM_RuneRock_02`))))
  (set `self.OutLocation` (`KismetMathLibrary.MakeTransform` _returnvalue_location _returnvalue_rotation _returnvalue_scale))
  (set `self.InLocation` (`KismetMathLibrary.MakeTransform` (- _returnvalue_location (0.0 0.0 70.0)) _returnvalue_rotation _returnvalue_scale)))

(event `self.SM_RuneRock_02.OnComponentHit`
  (params (HitComponent :type "PrimitiveComponent Object Reference") (OtherActor :type "Actor Object Reference") (OtherComp :type "PrimitiveComponent Object Reference") (NormalImpulse :type "Vector Structure") (Hit :type "HitResult Structure (by ref)"))
  (bind _returnvalue (`self.K2_GetActorLocation`))
  (`/Engine/EditorBlueprintResources/StandardMacros.DoOnce` false :!label _label
    (:`Completed`
      (`self.DisableInput` (`GameplayStatics.GetPlayerController` 0))
      (`GameplayStatics.PlaySoundAtLocation` "/Game/_ProjectContent/Audio/Stone_Slide_Cue.Stone_Slide_Cue" _returnvalue (struct) 1.0 1.0 0.0 null null null)
      (bind (_direction _stoneslide) (`Timeline|StoneActive` :!via `PlayFromStart`)
        (:`Update`
          (`SceneComponent.K2_SetRelativeTransform` (`self.SM_RuneRock_02`) (`KismetMathLibrary.TLerp` (`self.OutLocation`) (`self.InLocation`) _stoneslide) false false))
        (:`Finished`
          (`KismetSystemLibrary.Delay` 0.2)
          (`GameplayStatics.PlaySoundAtLocation` "/Game/_ProjectContent/Audio/Placing_Spacial_Cue.Placing_Spacial_Cue" _returnvalue (struct) 1.0 1.0 0.0 null null null)
          (`KismetSystemLibrary.Delay` 7.0)
          (`GameplayStatics.PlaySoundAtLocation` "/Game/_ProjectContent/Audio/Stone_Slide_Cue.Stone_Slide_Cue" (`self.K2_GetActorLocation`) (struct) 1.0 1.0 0.0 null null null)
          (bind (_direction_2 _stoneslide_2) (`Timeline|Timeline_0` :!via `ReverseFromEnd`)
            (:`Update`
              (`SceneComponent.K2_SetRelativeTransform` (`self.SM_RuneRock_02`) (`KismetMathLibrary.TLerp` (`self.OutLocation`) (`self.InLocation`) _stoneslide_2) false false))
            (:`Finished`
              (`self.EnableInput` (`GameplayStatics.GetPlayerController` 0))
              (goto _label :!via `Reset`))))))))

(fn `UserConstructionScript`)