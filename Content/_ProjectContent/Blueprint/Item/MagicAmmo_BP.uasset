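; MagicAmmo_BP is a pickup item that grants the player one unit of magic ammo.
; When its box overlaps the third-person character, it increments that character's MagicAmmo unless it has already reached the cap of five.
; On a successful pickup it plays a sound at the character's location and destroys itself, otherwise it stays in the world.
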(event `self.Box.OnComponentBeginOverlap`
  (params (OverlappedComponent :type "PrimitiveComponent Object Reference") (OtherActor :type "Actor Object Reference") (OtherComp :type "PrimitiveComponent Object Reference") (OtherBodyIndex :type Integer) (bFromSweep :type Boolean) (SweepResult :type "HitResult Structure (by ref)"))
  ;[1 1 1] PlusAmmo whenPlayer BeginOverlap
  (bind _asthird_person_character_bp (cast `/Game/_ProjectContent/Blueprint/ThirdPersonCharacter_BP` OtherActor))
  (bind _magicammo (`/Game/_ProjectContent/Blueprint/ThirdPersonCharacter_BP.MagicAmmo` _asthird_person_character_bp))
  (if (not (>= _magicammo 5))
    (set `/Game/_ProjectContent/Blueprint/ThirdPersonCharacter_BP.MagicAmmo` (+ _magicammo 1) _asthird_person_character_bp)
    (`GameplayStatics.PlaySoundAtLocation` "/Game/_ProjectContent/Audio/Pick_item1_Cue.Pick_item1_Cue" (`self.K2_GetActorLocation` _asthird_person_character_bp) (struct) 1.0 1.0 0.0 null null null)
    (`self.K2_DestroyActor`)))

(fn `UserConstructionScript`
  (`parent.UserConstructionScript`))