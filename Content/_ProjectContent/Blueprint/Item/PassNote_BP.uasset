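; PassNote_BP is a pickup note actor the player collects with the Interact input.
; Entering its box as ThirdPersonCharacter_BP enables input, shows a PickNote_UI prompt and opens a Gate; leaving reverses all three.
; Interacting while the gate is open sets HaveNote on the character and PlayerHaveNote on GameVar_Instance, plays a pickup sound and destroys the actor.
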(event `InputAction|Interact`
  (params (Key :type "Key Structure"))
  (:`Pressed`
    (`/Engine/EditorBlueprintResources/StandardMacros.Gate` true :!label _label
      (:`Exit`
        (set `/Game/_ProjectContent/Blueprint/ThirdPersonCharacter_BP.HaveNote?` true (stale `self.Box.OnComponentBeginOverlap` _asthird_person_character_bp))
        (`GameplayStatics.PlaySoundAtLocation` "/Game/_ProjectContent/Audio/Pick_item2_Cue.Pick_item2_Cue" (`self.K2_GetActorLocation`) (struct) 1.0 1.0 0.0 null null null)
        (bind _asgame_var_instance (cast `/Game/_ProjectContent/Blueprint/GameVar_Instance` (`GameplayStatics.GetGameInstance`)))
        (set `/Game/_ProjectContent/Blueprint/GameVar_Instance.PlayerHaveNote?` true _asgame_var_instance)
        (`self.K2_DestroyActor`)))))

(event `self.Box.OnComponentBeginOverlap`
  (params (OverlappedComponent :type "PrimitiveComponent Object Reference") (OtherActor :type "Actor Object Reference") (OtherComp :type "PrimitiveComponent Object Reference") (OtherBodyIndex :type Integer) (bFromSweep :type Boolean) (SweepResult :type "HitResult Structure (by ref)"))
  (bind _asthird_person_character_bp (cast `/Game/_ProjectContent/Blueprint/ThirdPersonCharacter_BP` OtherActor))
  (`self.EnableInput` (`GameplayStatics.GetPlayerController` 0))
  (bind _returnvalue (`|CreateWidget` "/Game/_ProjectContent/Widget/PickNote_UI.PickNote_UI_C"))
  (`UserWidget.AddToViewport` _returnvalue 0)
  (goto _label :!via `Open`))

(event `self.Box.OnComponentEndOverlap`
  (params (OverlappedComponent :type "PrimitiveComponent Object Reference") (OtherActor :type "Actor Object Reference") (OtherComp :type "PrimitiveComponent Object Reference") (OtherBodyIndex :type Integer))
  (cast `/Game/_ProjectContent/Blueprint/ThirdPersonCharacter_BP` OtherActor)
  (`self.DisableInput` (`GameplayStatics.GetPlayerController` 0))
  (`Widget.RemoveFromParent` (stale `self.Box.OnComponentBeginOverlap` _returnvalue))
  (goto _label :!via `Close`))

(fn `UserConstructionScript`)