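; Terrain puzzle piece that raises its static mesh when its TriggerOpened event fires.
; BeginPlay caches the mesh's relative transform as the start pose and derives a target pose offset upward on Z.
; TriggerOpened plays a trigger sound and runs a timeline that lerps the mesh between the two poses, then plays a stone-drop sound on finish.
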(event `self.ReceiveBeginPlay`
  (bind (_returnvalue_location _returnvalue_rotation _returnvalue_scale) (`KismetMathLibrary.BreakTransform` (`SceneComponent.GetRelativeTransform` (`self.StaticMesh`))))
  (set `self.OutPosition` (`KismetMathLibrary.MakeTransform` _returnvalue_location _returnvalue_rotation _returnvalue_scale))
  (set `self.InPosition` (`KismetMathLibrary.MakeTransform` (+ _returnvalue_location (0.0 0.0 295.0)) _returnvalue_rotation _returnvalue_scale)))

(event `TriggerOpened`
  (bind _returnvalue (`self.K2_GetActorLocation`))
  (`GameplayStatics.PlaySoundAtLocation` "/Game/_ProjectContent/Audio/terrainTrigger_Cue.terrainTrigger_Cue" _returnvalue (struct) 1.0 1.0 0.0 null null null)
  (bind (_direction _newtrack_0) (`Timeline|TerrainActive`)
    (:`Update`
      (`SceneComponent.K2_SetRelativeTransform` (`self.StaticMesh`) (`KismetMathLibrary.TLerp` (`self.OutPosition`) (`self.InPosition`) _newtrack_0) false false))
    (:`Finished`
      (`GameplayStatics.PlaySoundAtLocation` "/Game/_ProjectContent/Audio/StoneDrop_Cue.StoneDrop_Cue" _returnvalue (struct) 1.0 1.0 0.0 null null null))))

(fn `UserConstructionScript`)