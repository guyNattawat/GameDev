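; Enemy actor Blueprint with health, a health bar widget and slow self-regeneration.
; AnyDamage subtracts from current health and destroys the actor when it drops below zero.
; A sphere overlap shows the widget only while the ThirdPersonCharacter is inside.
; Tick pushes health into the cached widget and, below max, uses a Delay to regenerate health in small periodic steps.
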(event `self.ReceiveBeginPlay`
  (bind _asthird_person_character (cast `/Game/_ProjectContent/Blueprint/ThirdPersonCharacter` (`GameplayStatics.GetPlayerCharacter` 0)))
  (set `self.PlayerRef` _asthird_person_character)
  (bind _asai_health_ui (cast `/Game/_ProjectContent/Widget/AI_HealthUI` (`WidgetComponent.GetUserWidgetObject` (`self.HealthWidget`))))
  (set `self.Health Widget Ref` _asai_health_ui))

(event `self.ReceiveAnyDamage`
  (params (Damage :type "Float (single-precision)") (DamageType :type "DamageType Object Reference") (InstigatedBy :type "Controller Object Reference") (DamageCauser :type "Actor Object Reference"))
  ;[1 1 1] Health Reduce
  (set `self.HealthCurrent` (- (`self.HealthCurrent`) Damage))
  (if (< (`self.HealthCurrent`) 0.0)
    (`self.K2_DestroyActor`)))

(event `self.Sphere.OnComponentBeginOverlap`
  (params (OverlappedComponent :type "PrimitiveComponent Object Reference") (OtherActor :type "Actor Object Reference") (OtherComp :type "PrimitiveComponent Object Reference") (OtherBodyIndex :type Integer) (bFromSweep :type Boolean) (SweepResult :type "HitResult Structure (by ref)"))
  ;[1 1 1] Visibility Check Widget AI_Health
  (cast `/Game/_ProjectContent/Blueprint/ThirdPersonCharacter` OtherActor)
  (`SceneComponent.SetVisibility` (`self.HealthWidget`) true false))

(event `self.Sphere.OnComponentEndOverlap`
  (params (OverlappedComponent :type "PrimitiveComponent Object Reference") (OtherActor :type "Actor Object Reference") (OtherComp :type "PrimitiveComponent Object Reference") (OtherBodyIndex :type Integer))
  ;[1 1 1] Visibility Check Widget AI_Health
  (cast `/Game/_ProjectContent/Blueprint/ThirdPersonCharacter` OtherActor)
  (`SceneComponent.SetVisibility` (`self.HealthWidget`) false false))

(event `self.ReceiveTick`
  (params (DeltaSeconds :type "Float (single-precision)"))
  (`|ExecutionSequence`
    (:`then_0`
      (set `/Game/_ProjectContent/Widget/AI_HealthUI.Health` (`self.HealthCurrent`) (`self.Health Widget Ref`)))
    (:`then_1`
      (if (< (`self.HealthCurrent`) (`self.MaxHealth`))
        (`KismetSystemLibrary.Delay` 0.5)
        (set `self.HealthCurrent` (+ (`self.HealthCurrent`) 0.5))))))

(fn `UserConstructionScript`)